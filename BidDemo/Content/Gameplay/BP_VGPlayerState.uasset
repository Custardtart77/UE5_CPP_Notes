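; Player state Blueprint that carries the player's Health in and out of the save game object held by BP_VGGameInstance.
; On BeginPlay it copies Health from that save game into its own variable.
; When destroyed it writes the current Health back to the same object, without saving to disk itself.
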(event EventBeginPlay
  (bind _asbp_vggame_instance (Utilities|Casting|CastToBP_VGGameInstance (Game|GetGameInstance)))
  (Variables|Default|SetHealth (Variables|/Game/Gameplay/BP_VGSaveGame.BP_VGSaveGame_C|GetHealth (Variables|/Game/Gameplay/BP_VGGameInstance.BP_VGGameInstance_C|GetMySaveGame _asbp_vggame_instance))))

(event EventTick
  (params (DeltaSeconds :type Float%20%28single-precision%29)))

(event EventEndPlay
  (params (EndPlayReason :type EEndPlayReason%20Enum :default "Destroyed")))

(event EventDestroyed
  (bind _asbp_vggame_instance (Utilities|Casting|CastToBP_VGGameInstance (Game|GetGameInstance)))
  (Variables|/Game/Gameplay/BP_VGSaveGame.BP_VGSaveGame_C|SetHealth (Variables|/Game/Gameplay/BP_VGGameInstance.BP_VGGameInstance_C|GetMySaveGame _asbp_vggame_instance) (Variables|Default|GetHealth)))

(fn ConstructionScript)