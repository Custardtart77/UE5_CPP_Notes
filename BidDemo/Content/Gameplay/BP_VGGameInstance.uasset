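; BP_VGGameInstance is the game instance that holds the player's save object for the session.
; On Init it loads "PlayerSlot", casts it to BP_VGSaveGame and sets the user name to "PlayerOne".
; The branch condition is fixed to true, so the create-new-save path never runs and a failed cast leaves no save object set.
; On Shutdown it saves that object asynchronously to its stored slot and user index.
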(event EventInit
  (bind _returnvalue (SaveGame|LoadGamefromSlot "PlayerSlot"))
  (if true
    (bind _asbp_vgsave_game (Utilities|Casting|CastToBP_VGSaveGame _returnvalue))
    (bind _output_get (Variables|Default|SetMySaveGame _asbp_vgsave_game))
    (Variables|/Game/Gameplay/BP_VGSaveGame.BP_VGSaveGame_C|SetUserName _output_get "PlayerOne")
    (else
      (bind _returnvalue_2 (SaveGame|CreateSaveGameObject "/Game/Gameplay/BP_VGSaveGame.BP_VGSaveGame_C"))
      (bind _output_get_2 (Variables|Default|SetMySaveGame _returnvalue_2))
      (Variables|/Game/Gameplay/BP_VGSaveGame.BP_VGSaveGame_C|SetUserName _output_get_2 "PlayerOne")
      (Variables|/Game/Gameplay/BP_VGSaveGame.BP_VGSaveGame_C|SetUserIndex _output_get_2 0)
      (Variables|/Game/Gameplay/BP_VGSaveGame.BP_VGSaveGame_C|SetSaveSlotName _output_get_2 "PlayerSlot"))))

(event EventShutdown
  (bind _mysavegame (Variables|Default|GetMySaveGame))
  (|AsyncSaveGametoSlot _mysavegame (Variables|/Game/Gameplay/BP_VGSaveGame.BP_VGSaveGame_C|GetSaveSlotName _mysavegame) (Variables|/Game/Gameplay/BP_VGSaveGame.BP_VGSaveGame_C|GetUserIndex _mysavegame)))