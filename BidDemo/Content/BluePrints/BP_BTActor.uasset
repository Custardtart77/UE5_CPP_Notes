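; BP_BTActor is a trigger actor that shows a clickable button while an ALS character stands inside its box.
; On BeginPlay it creates a CustomButton widget and binds the button's click to a custom event.
; Box overlap begin adds the widget to the viewport and overlap end removes it.
; Clicking the button applies damage to the first player character, regardless of which character triggered the box.
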(event OnComponentBeginOverlap(Box)
  (params (OverlappedComponent :type Primitive%20Component%20Object%20Reference) (OtherActor :type Actor%20Object%20Reference) (OtherComp :type Primitive%20Component%20Object%20Reference) (OtherBodyIndex :type Integer) (bFromSweep :type Boolean) (SweepResult :type Hit%20Result%20Structure%20%28by%20ref%29))
  (Utilities|Casting|CastToALSCharacter OtherActor)
  (UserInterface|Viewport|AddtoViewport (Variables|Default|GetBT) 0))

(event OnComponentEndOverlap(Box)
  (params (OverlappedComponent :type Primitive%20Component%20Object%20Reference) (OtherActor :type Actor%20Object%20Reference) (OtherComp :type Primitive%20Component%20Object%20Reference) (OtherBodyIndex :type Integer))
  (Utilities|Casting|CastToALSCharacter OtherActor)
  (Widget|RemovefromParent (Variables|Default|GetBT)))

(event Custom|CustomEvent
  (Game|Damage|ApplyDamage (Game|GetPlayerCharacter 0) 2e+01 0 0))

(event EventBeginPlay
  (bind _returnvalue (UserInterface|CreateWidget "/Game/BluePrints/UI/CustomButton.CustomButton_C"))
  (bind _output_get (Variables|Default|SetBT _returnvalue))
  (EventDispatchers|BindEventtoOnClicked (Variables|/Game/BluePrints/UI/CustomButton.CustomButton_C|GetInteractionButton _output_get) (delegate Custom|CustomEvent)))

(event Collision|EventActorBeginOverlap
  (params (OtherActor :type Actor%20Object%20Reference)))

(event EventTick
  (params (DeltaSeconds :type Float%20%28single-precision%29)))

(fn ConstructionScript)