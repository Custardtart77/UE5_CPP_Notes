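; BP_torch is a torch actor that an ALS character can pick up through an on-screen button.
; On BeginPlay it creates a CustomButton widget with a bound click event, then shows or removes it as the character begins or ends overlap.
; The button click handler snaps the torch to TorchSocketName on the stored character's mesh, disables physics simulation on Mesh0 and removes the widget.
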(event Custom|OnButtonClick
  (Transformation|AttachComponentToComponent self (Variables|/Script/Engine.Character|GetMesh (Variables|Default|GetAs%20ALS%20Character%20BP)) (Variables|Default|GetTorchSocket%20Name) "SnapToTarget" "SnapToTarget" "SnapToTarget" true)
  (Physics|SetSimulatePhysics (Variables|Default|GetMesh_0) false)
  (Widget|RemovefromParent (Variables|Default|GetBT)))

(event EventBeginPlay
  (bind _returnvalue (UserInterface|CreateWidget "/Game/BluePrints/UI/CustomButton.CustomButton_C"))
  (bind _output_get (Variables|Default|SetBT _returnvalue))
  (EventDispatchers|BindEventtoOnClicked (Variables|/Game/BluePrints/UI/CustomButton.CustomButton_C|GetInteractionButton _output_get) (EventDispatchers|CreateEvent :!event Custom|OnButtonClick)))

(event Collision|EventActorBeginOverlap
  (params (OtherActor :type Actor%20Object%20Reference))
  (bind _asals_character_bp (Utilities|Casting|CastToALS_CharacterBP OtherActor))
  (Variables|Default|SetAs%20ALS%20Character%20BP _asals_character_bp)
  (UserInterface|Viewport|AddtoViewport (Variables|Default|GetBT) 0))

(event EventTick
  (params (DeltaSeconds :type Float%20%28single-precision%29)))

(event Collision|EventActorEndOverlap
  (params (OtherActor :type Actor%20Object%20Reference))
  (Utilities|Casting|CastToALS_CharacterBP OtherActor)
  (Widget|RemovefromParent (Variables|Default|GetBT)))

(fn ConstructionScript)